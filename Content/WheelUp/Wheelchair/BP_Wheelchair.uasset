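; Player-driven wheelchair vehicle pawn, playable in VR or on screen, that feeds input axes into its vehicle movement component.
; BeginPlay detects the HMD to set tracking and camera height (V toggles this), counts checkpoints and adds the GUI.
; R teleports to the checkpoint preceding the next one, falling back to PlayerStart.
; Hotkeys also load Tutorial or Restaurant, and a dev key alternately deactivates the main and side cameras without reactivating either.
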(event EventBeginPlay
  ;[1 1 1] Init
  (|CallParentFunction)
  ;;[1 1 1] Check if VR is connected
  (bind _hmddata (Class|HeadMountedDisplayFunctionLibrary|GetHMDData))
  (bind _output_get (Variables|Default|Setin%20VR%20Mode (.bValid (Utilities|Struct|BreakXRHMDData _hmddata))))
  (if _output_get
    (Utilities|SetVRMode)
    (else
      (Utilities|SetNotVRMode)))
  ;[1 1 1] Init Checkpoints
  (bind _outactors (Actor|GetAllActorsOfClass "/Game/WheelUp/Checkpoint/BP_Checkpoint.BP_Checkpoint_C"))
  (Variables|Default|SetTotal%20Checkpoint%20Count (Utilities|Array|Length _outactors))
  ;[1 1 1] Add Checkpoint UI
  (bind _returnvalue (UserInterface|CreateWidget "/Game/WheelUp/UI/GUI.GUI_C" (Game|GetPlayerController 0)))
  (UserInterface|Viewport|AddtoViewport _returnvalue 0))

(event Input|ActionEvents|InputActionHandbrake
  (params (Key :type Key%20Structure :default "None"))
  ;[1 1 1] Movement
  (:Pressed
    (Class|ChaosVehicleMovementComponent|SetHandbrakeInput (Variables|Default|GetVehicleMovementComponent) true))
  (:Released
    (Class|ChaosVehicleMovementComponent|SetHandbrakeInput (Variables|Default|GetVehicleMovementComponent) false)))

(event Input|AxisEvents|InputAxisBrake
  (params (AxisValue :type Float%20%28single-precision%29))
  ;[1 1 1] Movement
  (Class|ChaosVehicleMovementComponent|SetBrakeInput (Variables|Default|GetVehicleMovementComponent) AxisValue))

(event Input|AxisEvents|InputAxisMoveForward
  (params (AxisValue :type Float%20%28single-precision%29))
  ;[1 1 1] Movement
  (Class|ChaosVehicleMovementComponent|SetThrottleInput (Variables|Default|GetVehicleMovementComponent) AxisValue))

(event Input|AxisEvents|InputAxisSteerRight
  (params (AxisValue :type Float%20%28single-precision%29))
  ;[1 1 1] Movement
  (Class|ChaosVehicleMovementComponent|SetSteeringInput (Variables|Default|GetVehicleMovementComponent) AxisValue))

(event Input|KeyboardEvents|V
  (params (Key :type Key%20Structure :default "None"))
  ;[1 1 1] VR Mode Switch
  (:Pressed
    (if (Variables|Default|Getin%20VR%20Mode)
      (Utilities|SetNotVRMode)
      (else
        (Utilities|SetVRMode)))))

(event Input|KeyboardEvents|2
  (params (Key :type Key%20Structure :default "None"))
  ;[1 1 1] Level Switching
  (:Pressed
    (Game|OpenLevel(byObjectReference) "/Game/WheelUp/Maps/Restaurant.Restaurant")))

(event Input|KeyboardEvents|1
  (params (Key :type Key%20Structure :default "None"))
  ;[1 1 1] Level Switching
  (:Pressed
    (Game|OpenLevel(byObjectReference) "/Game/WheelUp/Maps/Tutorial.Tutorial")))

(event Input|KeyboardEvents|C
  (params (Key :type Key%20Structure :default "None"))
  ;[1 1 1] Dev: Toggle Side Camera
  (:Pressed
    (Utilities|FlowControl|FlipFlop
      (:A
        (Components|Activation|SetActive (Variables|Default|GetCamera) false false))
      (:B
        (Components|Activation|SetActive (Variables|Default|GetCameraSide) false false)))))

(event Input|KeyboardEvents|R
  (params (Key :type Key%20Structure :default "None"))
  ;[1 1 1] Quick Restart
  (:Pressed
    (bind _outactors (Actor|GetAllActorsOfClass "/Game/WheelUp/Checkpoint/BP_Checkpoint.BP_Checkpoint_C"))
    (for _array_element _outactors
      (if (Variables|/Game/WheelUp/Checkpoint/BP_Checkpoint.BP_Checkpoint_C|GetIs%20Next%20Checkpoint _array_element)
        (Utilities|IsValid (Variables|/Game/WheelUp/Checkpoint/BP_Checkpoint.BP_Checkpoint_C|GetLast%20Checkpoint _array_element)
          (:Is%20Valid
            (Transformation|SetActorLocation (Transformation|GetActorLocation (Variables|/Game/WheelUp/Checkpoint/BP_Checkpoint.BP_Checkpoint_C|GetLast%20Checkpoint _array_element)) false true))
          (:Is%20Not%20Valid
            (bind _returnvalue (Actor|GetActorOfClass "/Script/Engine.PlayerStart"))
            (Transformation|SetActorLocation (Transformation|GetActorLocation _returnvalue) false true)))
        (Audio|PlaySound2D "/Game/WheelUp/Sound/SFX/SFX_Quick_Restart.SFX_Quick_Restart" 1.0 1.0 0.0 0 0)))))

(fn ConstructionScript)