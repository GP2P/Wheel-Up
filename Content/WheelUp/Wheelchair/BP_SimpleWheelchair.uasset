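; Player wheelchair pawn for WheelUp, playable in VR or on desktop, with checkpoint restart, level hotkeys and camera toggle.
; Movement uses plain input or, with DynamicOn, a per-tick integration of force, torque and friction that auto-brakes without input.
; Hits are debounced by frame count, counted and flashed via post-process.
; Per-frame pose/input and events buffer in strings, appended on level switch to per-user CSVs created in the Construction Script.
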(event EventBeginPlay
  ;[1 1 1] Init
  (|CallParentFunction)
  ;;[1 1 1] Check if VR is connected
  (bind _hmddata (Class|HeadMountedDisplayFunctionLibrary|GetHMDData))
  (bind _output_get (Variables|Default|Setin%20VR%20Mode (.bValid (Utilities|Struct|BreakXRHMDData _hmddata))))
  (if _output_get
    (Utilities|SetVRMode)
    (else
      (Utilities|SetNotVRMode)))
  ;[1 1 1] Init Checkpoints
  (bind _outactors (Actor|GetAllActorsOfClass "/Game/WheelUp/Checkpoint/BP_Checkpoint.BP_Checkpoint_C"))
  (Variables|Checkpoint|SetTotal%20Checkpoint%20Count (Utilities|Array|Length _outactors))
  ;[1 1 1] Add Checkpoint UI
  (bind _returnvalue (UserInterface|CreateWidget "/Game/WheelUp/UI/GUI.GUI_C" (Game|GetPlayerController 0)))
  (UserInterface|Viewport|AddtoViewport _returnvalue 0)
  ;[1 1 1] Init Dynamics
  (CallFunction|InitDynamics)
  ;[1 1 1] Clear camera post processing
  (Class|CameraComponent|SetPostProcessBlendWeight (Variables|Default|GetCamera) 0.0))

(event Collision|EventHit
  (params (MyComp :type Primitive%20Component%20Object%20Reference) (Other :type Actor%20Object%20Reference) (OtherComp :type Primitive%20Component%20Object%20Reference) (bSelfMoved :type Boolean) (HitLocation :type Vector :default "0, 0, 0") (HitNormal :type Vector :default "0, 0, 0") (NormalImpulse :type Vector :default "0, 0, 0") (Hit :type Hit%20Result%20Structure%20%28by%20ref%29))
  ;[1 1 1] Collision Detection
  (|CallParentFunction OtherComp Other 0 bSelfMoved NormalImpulse "0, 0, 0" "0, 0, 0" Hit)
  ;;[1 1 1] Spam Prevention
  (if (>= (- (Utilities|GetFrameCount) (Variables|Collision|GetLast%20Collision%20Frame)) 10)
    (bind _result (Math|Integer|IncrementInt (Variables|Collision|GetCollision%20Count))
      (:%20%20
        (Utilities|AppendEventData "CC" _result)
        (Development|PrintString (Utilities|String|Append "Collision Detected: " (Utilities|String|ToString(Integer) (Variables|Collision|GetCollision%20Count))))
        (bind _delta (Timeline|Collision PlayFromStart)
          (:Update
            (Class|CameraComponent|SetPostProcessBlendWeight (Variables|Default|GetCamera) _delta))))))
  (Variables|Collision|SetLast%20Collision%20Frame (Utilities|GetFrameCount)))

(event EventTick
  (params (DeltaSeconds :type Float%20%28single-precision%29))
  ;[1 1 1] Append Data Each Frame
  (|CallParentFunction DeltaSeconds)
  ;;[1 1 1] Dynamics
  (if (Variables|Default|GetDynamic%20On)
    (CallFunction|PrintInput)
    (CallFunction|UpdatePosition DeltaSeconds))
  (Utilities|AppendFrameData))

(event Input|AxisEvents|InputAxisMoveForward
  (params (AxisValue :type Float%20%28single-precision%29))
  ;[1 1 1] Movement
  (if (not (Variables|Default|GetDynamic%20On))
    (Pawn|Input|AddMovementInput (Math|Vector|GetForwardVector (Math|Rotator|MakeRotator 0.0 0.0 (.Yaw (Math|Rotator|BreakRotator (Pawn|GetControlRotation :!class /Script/Engine.Pawn))))) AxisValue false)))

(event Input|AxisEvents|InputAxisSteerRight
  (params (AxisValue :type Float%20%28single-precision%29))
  ;[1 1 1] Movement
  (if (not (Variables|Default|GetDynamic%20On))
    (Pawn|Input|AddControllerYawInput AxisValue)))

(event Input|KeyboardEvents|SpaceBar
  (params (Key :type Key%20Structure :default "None"))
  ;[1 1 1] Break with Space Key (not active)
)

(event Input|KeyboardEvents|2
  (params (Key :type Key%20Structure :default "None"))
  ;[1 1 1] Level Switching
  (:Pressed
    (Utilities|AppendEventData "LS" 2)
    (CallFunction|AppendDataFiles)
    (Game|OpenLevel(byObjectReference) "/Game/WheelUp/Maps/Restaurant.Restaurant")))

(event Input|KeyboardEvents|1
  (params (Key :type Key%20Structure :default "None"))
  ;[1 1 1] Level Switching
  (:Pressed
    (Utilities|AppendEventData "LS" 1)
    (CallFunction|AppendDataFiles)
    (Game|OpenLevel(byObjectReference) "/Game/WheelUp/Maps/Tutorial.Tutorial")))

(event Input|KeyboardEvents|C
  (params (Key :type Key%20Structure :default "None"))
  ;[1 1 1] Dev: Toggle Side Camera
  (:Pressed
    (Utilities|FlowControl|FlipFlop
      (:A
        (Components|Activation|SetActive (Variables|Default|GetCamera) false false)
        (Utilities|AppendEventData "C"))
      (:B
        (Components|Activation|SetActive (Variables|Default|GetCameraSide) false false)
        (Utilities|AppendEventData "C" 1)))))

(event Input|KeyboardEvents|R
  (params (Key :type Key%20Structure :default "None"))
  ;[1 1 1] Quick Restart
  (:Pressed
    ;;[1 1 1] Find next Checkpoint
    (bind _outactors (Actor|GetAllActorsOfClass "/Game/WheelUp/Checkpoint/BP_Checkpoint.BP_Checkpoint_C"))
    (for (_array_element _array_index) _outactors
      (if (Variables|/Game/WheelUp/Checkpoint/BP_Checkpoint.BP_Checkpoint_C|GetIs%20Next%20Checkpoint _array_element)
        ;;[1 1 1] Teleport to checkpoint before it, if exists, else to playerstart
        (Utilities|IsValid (Variables|/Game/WheelUp/Checkpoint/BP_Checkpoint.BP_Checkpoint_C|GetLast%20Checkpoint _array_element)
          (:Is%20Valid
            (Transformation|SetActorLocation (Transformation|GetActorLocation (Variables|/Game/WheelUp/Checkpoint/BP_Checkpoint.BP_Checkpoint_C|GetLast%20Checkpoint _array_element)) false true))
          (:Is%20Not%20Valid
            (bind _returnvalue (Actor|GetActorOfClass "/Script/Engine.PlayerStart"))
            (Transformation|SetActorLocation (Transformation|GetActorLocation _returnvalue) false true)))
        (Audio|PlaySound2D "/Game/WheelUp/Sound/SFX/SFX_Quick_Restart.SFX_Quick_Restart" 1.0 1.0 0.0 0 0)
        (Utilities|AppendEventData "QR" _array_index)))))

(event Input|KeyboardEvents|V
  (params (Key :type Key%20Structure :default "None"))
  ;[1 1 1] VR Mode Switch
  (:Pressed
    (if (Variables|Default|Getin%20VR%20Mode)
      (Utilities|AppendEventData "VR" 1)
      (else
        (Utilities|AppendEventData "VR")))))

(event Input|KeyboardEvents|3
  (params (Key :type Key%20Structure :default "None"))
  ;[1 1 1] Level Switching
  (:Pressed
    (Utilities|AppendEventData "LS" 3)
    (CallFunction|AppendDataFiles)
    (Game|OpenLevel(byObjectReference) "/Game/WheelUp/Maps/WorkSpace.WorkSpace")))

(event Input|KeyboardEvents|4
  (params (Key :type Key%20Structure :default "None"))
  ;[1 1 1] Level Switching
  (:Pressed
    (Utilities|AppendEventData "LS" 4)
    (CallFunction|AppendDataFiles)
    (Game|OpenLevel(byObjectReference) "/Game/WheelUp/Maps/AlexOffice.AlexOffice")))

(fn ConstructionScript
  (|GenerateFileNames)
  (|CreateFiles)
  (|InitFiles))

(fn AppendDataFiles
  (bind _frames_file_name (Variables|Data|GetFrames%20File%20Name))
  (bind _events_file_name (Variables|Data|GetEvents%20File%20Name))
  (bind _returnvalue (Class|FileSDKBPLibrary|WriteStringtoFile _frames_file_name (Variables|Data|GetFrames%20Data%20String) true "AutoDetect"))
  (if _returnvalue
    (Variables|Data|SetFrames%20Data%20String "")
    (else
      (Development|PrintString (Utilities|String|Append "Error Writing To FIle: " _frames_file_name) true true "(R=1.000000,G=0.012817,B=0.000000,A=1.000000)" 2e+01)))
  (bind _returnvalue_2 (Class|FileSDKBPLibrary|WriteStringtoFile _events_file_name (Variables|Data|GetEvents%20Data%20String) true "AutoDetect"))
  (if _returnvalue_2
    (Variables|Data|SetEvents%20Data%20String "")
    (else
      (Development|PrintString (Utilities|String|Append "Error Writing To FIle: " _events_file_name) true true "(R=1.000000,G=0.012817,B=0.000000,A=1.000000)" 2e+01)))
  (return (and _returnvalue_2 _returnvalue)))

(fn InitDynamics
  (bind _returnvalue (Transformation|GetActorTransform))
  (bind (_location _rotation) (Math|Transform|BreakTransform _returnvalue))
  ;[1 1 1] Init Dynamics
  (Variables|Locamotion|SetCurrent%20Friction%20Coefficient (Variables|PhysicsConstants|GetRolling%20Friction%20Coefficient))
  (bind _output_get (Variables|Locamotion|SetXn _location))
  (Development|PrintString (Utilities|String|BuildString(Vector) "Xn init to: " "" _output_get) true true "(R=0.000000,G=0.660000,B=1.000000,A=1.000000)" 1e+01)
  (Variables|Locamotion|SetTHn (Math|Vector|MakeVector 0.0 0.0 (.Yaw (Math|Rotator|BreakRotator _rotation))))
  (Development|PrintString (Utilities|String|BuildString(Vector) "THn init to: " "" (Math|Rotator|GetRotationXVector _rotation)) true true "(R=0.000000,G=0.660000,B=1.000000,A=1.000000)" 1e+01))

(fn UpdatePosition
  (params (InputPin :type Float%20%28single-precision%29))
  ;[1 1 1] If no Input, Auto Break
  (if (|InputNearZero (Input|AxisValues|GetMoveForward) (Input|AxisValues|GetSteerRight))
    (Variables|Locamotion|SetCurrent%20Friction%20Coefficient (Variables|PhysicsConstants|GetSlideing%20Friction%20Coefficient))
    (else
      (Variables|Locamotion|SetCurrent%20Friction%20Coefficient (Variables|PhysicsConstants|GetRolling%20Friction%20Coefficient))))
  ;[1 1 1] Linear Force + Friction
  (bind _output_get (Variables|Locamotion|SetVn+1 (|CalcVn+1(m)_2 InputPin)))
  (Variables|Locamotion|SetVn _output_get)
  (bind _output_get_2 (Variables|Locamotion|SetXn+1 (.Xn+1 (|CalcXn+1(m->cm)_2 _output_get InputPin))))
  (Variables|Locamotion|SetXn _output_get_2)
  ;[1 1 1] Roation + Friction
  (bind _output_get_3 (Variables|Locamotion|SetWn+1 (|CalcWn+1(rad)_2 InputPin)))
  (Variables|Locamotion|SetWn _output_get_3)
  (bind _output_get_4 (Variables|Locamotion|SetTHn+1 (.THn+1 (|CalcTHn+1_2 _output_get_3 InputPin))))
  (Variables|Locamotion|SetTHn _output_get_4)
  (Pawn|Input|AddControllerYawInput (.Z (Math|Vector|BreakVector (.DTH (|CalcTHn+1_2 _output_get_3 InputPin)))))
  (Transformation|SetActorLocationAndRotation _output_get_2 (Pawn|GetControlRotation :!class /Script/Engine.Pawn)))

(fn PrintInput
  (Development|PrintString (Class|KismetStringLibrary|BuildStringDouble "X: " "" (Input|AxisValues|GetMoveForward)))
  (Development|PrintString (Class|KismetStringLibrary|BuildStringDouble "Y :" "" (Input|AxisValues|GetSteerRight))))